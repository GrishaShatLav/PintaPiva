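; BP_Platform is a moving platform that disables the player's hook while the player overlaps it.
; Its construction script sets the InterpToMovement control points from relative start and end locations and applies the Duration.
; Begin and end overlap events call ChangeHookAccess on BP_PlayerCharacter to turn hook access off and back on.
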(event `self.ReceiveActorBeginOverlap`
  (params (OtherActor :type "Actor Object Reference"))
  (bind _asbp_player_character (cast `/Game/PlayerCharacter/BP_PlayerCharacter` OtherActor))
  (`/Game/Andrey/Blueprints/BPI_Player.ChangeHookAccess` _asbp_player_character false))

(event `self.ReceiveActorEndOverlap`
  (params (OtherActor :type "Actor Object Reference"))
  (bind _asbp_player_character (cast `/Game/PlayerCharacter/BP_PlayerCharacter` OtherActor))
  (`/Game/Andrey/Blueprints/BPI_Player.ChangeHookAccess` _asbp_player_character true))

(fn `UserConstructionScript`
  (bind _interptomovement (`self.InterpToMovement`))
  (set `InterpToMovementComponent.ControlPoints` (`|MakeArray` (make `InterpControlPoint` (`self.StartLocation`)) (make `InterpControlPoint` (`self.EndLocation`))) _interptomovement)
  (set `InterpToMovementComponent.Duration` (`self.Duration`) _interptomovement))