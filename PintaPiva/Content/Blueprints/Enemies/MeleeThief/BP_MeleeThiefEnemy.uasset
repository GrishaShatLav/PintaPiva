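; Melee thief enemy that can steal one of the player's input keys when its weapon hits.
; Attack opens a 0.8-second DidItHitActor trace window on the Weapon component; its montage call is unwired.
; Player-tagged hits that pass a random roll against HitChance (higher values mean fewer steals) call HitAI on the first-person character.
; The returned key selects a matching Key actor to spawn, targeting the thief with radius and rotation speed set.
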(event `Event Attack`
  (bind _didithitactor (`self.DidItHitActor`))
  (`DidItHitActorComponent.ToggleTraceCheck` _didithitactor true)
  (`KismetSystemLibrary.Delay` 0.8)
  (`DidItHitActorComponent.ToggleTraceCheck` _didithitactor false))

(event `self.DidItHitActor.OnItemAdded`
  (params (LastItem :type "HitResult Structure"))
  (bind _returnvalue (`self.GetTransform`))
  (if (`self.ActorHasTag` LastItem_HitActor "Player")
    (if (>= (`KismetMathLibrary.RandomFloatInRange` 0.0 100.0) (`self.HitChance`))
      (`|ExecutionSequence`
        (:`then_0`
          (bind _asbp_first_person_character (cast `/Game/FirstPerson/Blueprints/BP_FirstPersonCharacter` LastItem_HitActor))
          (bind _stolenbutton (`/Game/Andrey/Blueprints/BPI_Player.HitAI` _asbp_first_person_character))
          (switch `/Game/Blueprints/Enums/EPhysicalButtons` _stolenbutton
            (:`NewEnumerator0`
              (bind _returnvalue_2 (`|SpawnActorFromClass` "/Game/Vadim/Keyboard/Key_w.Key_w_C" _returnvalue "Undefined" "OverrideRootScale" null null))
              (set `/Game/Vadim/Keyboard/Key.ActorTarget` self _returnvalue_2)
              (set `/Game/Vadim/Keyboard/Key.Radius` 200.0 _returnvalue_2)
              (set `/Game/Vadim/Keyboard/Key.Rotation speed` 20.0 _returnvalue_2))
            (:`NewEnumerator1`
              (bind _returnvalue_3 (`|SpawnActorFromClass` "/Game/Vadim/Keyboard/Key_a.Key_a_C" _returnvalue "Undefined" "OverrideRootScale" null null))
              (set `/Game/Vadim/Keyboard/Key.ActorTarget` self _returnvalue_3)
              (set `/Game/Vadim/Keyboard/Key.Radius` 200.0 _returnvalue_3)
              (set `/Game/Vadim/Keyboard/Key.Rotation speed` 20.0 _returnvalue_3))
            (:`NewEnumerator2`
              (bind _returnvalue_4 (`|SpawnActorFromClass` "/Game/Vadim/Keyboard/Key_s.Key_s_C" _returnvalue "Undefined" "OverrideRootScale" null null))
              (set `/Game/Vadim/Keyboard/Key.ActorTarget` self _returnvalue_4)
              (set `/Game/Vadim/Keyboard/Key.Radius` 200.0 _returnvalue_4)
              (set `/Game/Vadim/Keyboard/Key.Rotation speed` 20.0 _returnvalue_4))
            (:`NewEnumerator3`
              (bind _returnvalue_5 (`|SpawnActorFromClass` "/Game/Vadim/Keyboard/Key_d.Key_d_C" _returnvalue "Undefined" "OverrideRootScale" null null))
              (set `/Game/Vadim/Keyboard/Key.ActorTarget` self _returnvalue_5)
              (set `/Game/Vadim/Keyboard/Key.Radius` 200.0 _returnvalue_5)
              (set `/Game/Vadim/Keyboard/Key.Rotation speed` 20.0 _returnvalue_5))
            (:`NewEnumerator4`
              (bind _returnvalue_6 (`|SpawnActorFromClass` "/Game/Vadim/Keyboard/Key_lmb.Key_lmb_C" _returnvalue "Undefined" "OverrideRootScale" null null))
              (set `/Game/Vadim/Keyboard/Key.ActorTarget` self _returnvalue_6)
              (set `/Game/Vadim/Keyboard/Key.Radius` 200.0 _returnvalue_6)
              (set `/Game/Vadim/Keyboard/Key.Rotation speed` 20.0 _returnvalue_6))
            (:`NewEnumerator5`
              (bind _returnvalue_7 (`|SpawnActorFromClass` "/Game/Vadim/Keyboard/Key_rmb.Key_rmb_C" _returnvalue "Undefined" "OverrideRootScale" null null))
              (set `/Game/Vadim/Keyboard/Key.ActorTarget` self _returnvalue_7)
              (set `/Game/Vadim/Keyboard/Key.Radius` 200.0 _returnvalue_7)
              (set `/Game/Vadim/Keyboard/Key.Rotation speed` 20.0 _returnvalue_7))
            (:`NewEnumerator6`
              (bind _returnvalue_8 (`|SpawnActorFromClass` "/Game/Vadim/Keyboard/Key_shift.Key_shift_C" _returnvalue "Undefined" "OverrideRootScale" null null))
              (set `/Game/Vadim/Keyboard/Key.ActorTarget` self _returnvalue_8)
              (set `/Game/Vadim/Keyboard/Key.Radius` 200.0 _returnvalue_8)
              (set `/Game/Vadim/Keyboard/Key.Rotation speed` 20.0 _returnvalue_8))
            (:`NewEnumerator7`
              (bind _returnvalue_9 (`|SpawnActorFromClass` "/Game/Vadim/Keyboard/Key_space.Key_space_C" _returnvalue "Undefined" "OverrideRootScale" null null))
              (set `/Game/Vadim/Keyboard/Key.ActorTarget` self _returnvalue_9)
              (set `/Game/Vadim/Keyboard/Key.Radius` 200.0 _returnvalue_9)
              (set `/Game/Vadim/Keyboard/Key.Rotation speed` 20.0 _returnvalue_9))))))))

(fn `UserConstructionScript`
  (`parent.UserConstructionScript`)
  (`DidItHitActorComponent.SetupVariables` (`self.DidItHitActor`) (`self.Weapon`) null))