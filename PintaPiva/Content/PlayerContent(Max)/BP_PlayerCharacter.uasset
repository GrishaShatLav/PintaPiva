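; BP_PlayerCharacter is a player character with a grappling move triggered by the right mouse button.
; A visibility sphere trace along the camera's forward vector finds the target, pulled back from the hit along that vector.
; The Grappling event records the start location, then a timeline lerps the actor to the target, setting location without sweep, so collisions along the path are ignored.
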(event `self.ReceiveBeginPlay`)

(event `Key|RightMouseButton`
  (params (Key :type "Key Structure"))
  (bind _camera (`self.Camera`))
  (bind _returnvalue (`SceneComponent.K2_GetComponentLocation` _camera))
  (bind _returnvalue_2 (`SceneComponent.GetForwardVector` _camera))
  (:`Pressed`
    (bind (_outhit _returnvalue_3) (`KismetSystemLibrary.SphereTraceSingle` _returnvalue (+ _returnvalue (* _returnvalue_2 2000.0)) 0.0 "TraceTypeQuery1"))
    (if _returnvalue_3
      (`self.Grappling` (+ (`.Location` (`GameplayStatics.BreakHitResult` _outhit)) (* _returnvalue_2 -55.0))))))

(event `Grappling`
  (params (AttachPoint :type "Vector Structure"))
  (set `self.StartPoint` (`self.K2_GetActorLocation`))
  (bind (_direction _alpha) (`Timeline|Grapple` :!via `PlayFromStart`)
    (:`Update`
      (`self.K2_SetActorLocation` (`KismetMathLibrary.VLerp` (`self.StartPoint`) AttachPoint _alpha)))))

(fn `UserConstructionScript`)