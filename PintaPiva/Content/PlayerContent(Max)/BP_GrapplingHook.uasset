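; Grappling hook actor that draws the rope as a spline mesh shooting from a character toward a target point.
; SetPoints stores the character and plays the Hook timeline, lerping the mesh end from character to target in the hook's local space.
; Once spawned, Tick keeps resetting the mesh start, but converts the character's location with the character's own transform rather than the hook's.
; It contains no character movement logic.
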(event `self.ReceiveTick`
  (params (DeltaSeconds :type "Float (single-precision)"))
  (bind _character_ref (`self.Character Ref`))
  (if (`self.isSpawned`)
    (`SplineMeshComponent.SetStartPosition` (`self.SplineMeshComponent`) (`KismetMathLibrary.InverseTransformLocation` (`self.GetTransform` _character_ref) (`self.K2_GetActorLocation` _character_ref)) true)))

(event `SetPoints`
  (params (EndPoint :type "Vector Structure") (CharacterRef :type "/Game/FirstPerson/Blueprints/BP_FirstPersonCharacter Object Reference"))
  (bind _returnvalue (`self.GetTransform`))
  (bind _returnvalue_2 (`KismetMathLibrary.InverseTransformLocation` _returnvalue (`self.K2_GetActorLocation` CharacterRef)))
  (set `self.Character Ref` CharacterRef)
  (bind (_direction _alpha) (`Timeline|Hook` :!via `PlayFromStart`)
    (:`Update`
      (`SplineMeshComponent.SetStartAndEnd` (`self.SplineMeshComponent`) _returnvalue_2 (0.0 0.0 0.0) (`KismetMathLibrary.VLerp` _returnvalue_2 (`KismetMathLibrary.InverseTransformLocation` _returnvalue EndPoint) _alpha) (0.0 0.0 0.0) true)
      (set `self.isSpawned` true))))

(fn `UserConstructionScript`)